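; Bridge 24x24 T-junction piece for the procedural road generator, with all of its logic in the construction script.
; It converts the SelectConnectors choice to the integer connector ID to connect, then runs the parent construction script.
; It also randomly gives DecalC a road-line or arrow material and shows Decal2 and Decal3 only when UseSmallCross is set.
; The event graph holds only disabled default events.
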(fn `UserConstructionScript`
  (bind _decal2 (`self.Decal2`))
  (set `self.Connectors ID To Connect` (`KismetMathLibrary.Conv_ByteToInt` (`self.Select Connectors`)))
  (`DecalComponent.SetDecalMaterial` (`self.Decal_c`) (select `bool` (`KismetMathLibrary.RandomBool`) :`false` "/Game/ProceduralRoadGenerator/Material/Road_Asphalt/Arrow_road_01_Inst.Arrow_road_01_Inst" :`true` "/Game/ProceduralRoadGenerator/Material/Road_Asphalt/RoadLines014_Inst.RoadLines014_Inst" :!type "MaterialInterface Object Reference"))
  (`parent.UserConstructionScript`)
  (if (`self.Use Small Cross`)
    (`SceneComponent.SetVisibility` _decal2 true false)
    (`SceneComponent.SetVisibility` (`self.Decal3`) true false)
    (else
      (`SceneComponent.SetVisibility` _decal2 false false)
      (`SceneComponent.SetVisibility` (`self.Decal3`) false false))))
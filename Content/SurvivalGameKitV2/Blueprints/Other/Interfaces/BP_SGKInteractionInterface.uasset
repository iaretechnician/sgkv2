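; Blueprint interface from Survival Game Kit V2 that defines the contract for world objects the player can interact with.
; It covers interaction permission, available actions, display name, and starting or ending interactions using the player inventory.
; Further functions expose item data, amount, mesh and dropping, plus code entry with verified-player tracking.
; Turned-on effect and player proximity notifications round out the contract, which holds only empty default stubs.
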(fn `SGK AllowInteraction`
  (returns (AllowInteraction :type Boolean))
  (return false))

(fn `SGK CodeCheck`
  (params (Code :type Text))
  (returns (CodeAccepted :type Boolean))
  (return false))

(fn `SGK DropItem`
  (params (InvItem :type "/Game/SurvivalGameKitV2/Blueprints/Other/Structs/S_InvItem Structure") (Dropped :type Boolean) (Spawned :type Boolean) (SaveLoaded :type Boolean))
  (returns (ReturnValue :type Boolean))
  (return false))

(fn `SGK EndInteraction`
  (params (PlayerInventory :type "/Game/SurvivalGameKitV2/Components/BP_PlayerInventory Object Reference"))
  (returns (ReturnValue :type Boolean))
  (return false))

(fn `SGK GetVerifiedPlayers`
  (returns (VerifiedPlayers :type "Array of Text"))
  (return))

(fn `SGK Interact`
  (params (PlayerInventory :type "/Game/SurvivalGameKitV2/Components/BP_PlayerInventory Object Reference") (Action :type "/Game/SurvivalGameKitV2/Blueprints/Other/Enum/E_WorldActions Enum" :default "NewEnumerator0"))
  (returns (ReturnValue :type Boolean))
  (return false))

(fn `SGK InteractName`
  (returns (InteractName :type Text))
  (return ""))

(fn `SGK InvItem`
  (returns (IsItem :type Boolean) (InvItem :type "/Game/SurvivalGameKitV2/Blueprints/Other/Structs/S_InvItem Structure"))
  (return false))

(fn `SGK ItemAmount`
  (returns (Amount :type Integer))
  (return 0))

(fn `SGK Mesh`
  (returns (Mesh :type "PrimitiveComponent Object Reference"))
  (return null))

(fn `SGK PlayerInProximity`)

(fn `SGK PlayerOutProximity`)

(fn `SGK PossibleActions`
  (params (PlayerInventory :type "/Game/SurvivalGameKitV2/Components/BP_PlayerInventory Object Reference"))
  (returns (ActionsFound :type Boolean) (PossibleActions :type "Array of /Game/SurvivalGameKitV2/Blueprints/Other/Structs/S_WorldAction Structure"))
  (return false))

(fn `SGK SetVerifiedPlayers`
  (params (VerifiedPlayers :type "Array of Text")))

(fn `SGK TurnedOnEffect`
  (params (TurnedOn :type Boolean)))

(fn `SGK UpdateCode`
  (params (Code :type Text))
  (returns (ReturnValue :type Boolean))
  (return false))

(fn `SGK VerifyPlayer`
  (params (Text :type Text))
  (returns (ReturnValue :type Boolean))
  (return false))
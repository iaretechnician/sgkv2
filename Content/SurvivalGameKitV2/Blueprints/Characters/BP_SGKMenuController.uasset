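; BP_SGKMenuController is a menu controller for the Survival Game Kit that sets up input and shows the main menu when play begins.
; For the local controller, it adds the kit's bindable Enhanced Input config, then has BP_SGKGameInstance load controls if the cast succeeds.
; It then creates and stores the menu widget, adds it to the viewport and shows the mouse cursor.
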(fn `UserConstructionScript`)